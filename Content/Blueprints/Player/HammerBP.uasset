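; HammerBP is a player-related hammer actor that trails a flickering lightning effect.
; On BeginPlay it spawns a separate NiagaraActor with the LightningHammer system and sets Beam Start to the hammer's location.
; Each Tick it randomly jitters Beam End around the hammer's X/Y, leaving Z unwired, then refreshes Beam Start.
; OnDestroy destroys the spawned effect actor.
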(event EventBeginPlay
  (bind _self self)
  (bind _returnvalue (Transformation|GetActorLocation _self))
  (bind _returnvalue_2 (Game|SpawnActorfromClass "/Script/Niagara.NiagaraActor" (Transformation|GetActorTransform _self) "Undefined" _self 0))
  (bind _output_get (Variables|Default|SetlightningEffect _returnvalue_2))
  (Class|NiagaraComponent|SetAsset (Variables|/Script/Niagara.NiagaraActor|GetNiagaraComponent _output_get) "/Game/Effects/VFX/LightningHammer.LightningHammer" true)
  (Niagara|SetNiagaraVariable(Vector3) (Variables|/Script/Niagara.NiagaraActor|GetNiagaraComponent (Variables|Default|GetlightningEffect)) "Beam Start" (Math|Vector|MakeVector (.x _returnvalue) (.y _returnvalue) (.z _returnvalue))))

(event Collision|EventActorBeginOverlap
  (params (OtherActor :type Actor%20Object%20Reference)))

(event EventTick
  (params (DeltaSeconds :type Float%20%28single-precision%29))
  (bind _self self)
  (bind _lightningeffect (Variables|Default|GetlightningEffect))
  (bind _returnvalue (Transformation|GetActorLocation _self))
  (bind _niagaracomponent (Variables|/Script/Niagara.NiagaraActor|GetNiagaraComponent _lightningeffect))
  (Niagara|SetNiagaraVariable(Vector3) _niagaracomponent "Beam End" (Math|Vector|MakeVector (+ (.x _returnvalue) (Math|Random|RandomFloatinRange -75.0 75.0)) (+ (.y _returnvalue) (Math|Random|RandomFloatinRange -75.0 75.0)) 0.0))
  (Niagara|SetNiagaraVariable(Vector3) _niagaracomponent "Beam Start" (Math|Vector|MakeVector (.x _returnvalue) (.y _returnvalue) (.z _returnvalue))))

(event EventOnDestroy
  (Actor|DestroyActor (Variables|Default|GetlightningEffect)))

(fn ConstructionScript)